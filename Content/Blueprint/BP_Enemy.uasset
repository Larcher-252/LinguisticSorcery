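; BP_Enemy is a flipbook-animated enemy with a health bar widget, for a side-scroller game.
; AddDamage clamps HP at zero, updates the widget's HP percent and triggers Death when HP reaches zero.
; UpdateAnimation switches idle, attack and death flipbooks from AnimState, or stops the sprite when StopGame is set.
; The death branch waits briefly, asks GM_SideScroller to spawn a new enemy, then destroys the actor.
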(event `self.ReceiveBeginPlay`
  (bind _asw_enemy_hp (cast `/Game/Blueprint/UI/W_Enemy_HP` (`WidgetComponent.GetUserWidgetObject` (`self.Widget`))))
  (set `self.HP_Ref` _asw_enemy_hp)
  (`self.Add_Damage` 0.0))

(event `UpdateAnimation`
  (if (not (`self.StopGame`))
    (if (not (`PaperFlipbookComponent.IsPlaying` (`self.Sprite`)))
      (`PaperFlipbookComponent.Play` (`self.Sprite`)))
    (switch `/Game/Blueprint/Enum_Player_AnimState` (`self.AnimState`)
      (:`NewEnumerator0`
        (`PaperFlipbookComponent.SetFlipbook` (`self.Sprite`) "/Game/Assets/Sprites/Enemy/Idle/FB_Enemy_Idle.FB_Enemy_Idle")
        (`PaperFlipbookComponent.SetLooping` (`self.Sprite`) true))
      (:`NewEnumerator1`
        (`PaperFlipbookComponent.SetFlipbook` (`self.Sprite`) "/Game/Assets/Sprites/Enemy/Attack/FB_Enemy_Attack.FB_Enemy_Attack")
        (`PaperFlipbookComponent.SetLooping` (`self.Sprite`) false))
      (:`NewEnumerator2`
        (`PaperFlipbookComponent.SetFlipbook` (`self.Sprite`) "/Game/Assets/Sprites/Enemy/Death/FB_Enemy_Dead.FB_Enemy_Dead")
        (`PaperFlipbookComponent.SetLooping` (`self.Sprite`) false)
        (`KismetSystemLibrary.Delay` 2.0)
        (bind _asgm_side_scroller (cast `/Game/Blueprint/GM_SideScroller` (`GameplayStatics.GetGameMode`)))
        (`/Game/Blueprint/GM_SideScroller.SpawnNewEnemy` _asgm_side_scroller)
        (`self.K2_DestroyActor`)))
    (else
      (`PaperFlipbookComponent.Stop` (`self.Sprite`)))))

(fn `Add_Damage`
  (params (InDamage :type "Float (double-precision)"))
  (locals (NewHP :type "Float (double-precision)"))
  (bind _output_get (set `local.NewHP` (- (`self.HP_current`) InDamage)))
  (if (< _output_get 0.0)
    (set `local.NewHP` 0.0))
  (set `self.HP_current` (`local.NewHP`))
  (set `/Game/Blueprint/UI/W_Enemy_HP.HP_Percent` (/ (`self.HP_current`) (`self.HP_max`)) (`self.HP_Ref`))
  (if (== 0.0 (`self.HP_current`))
    (`self.Death`)))

(fn `Death`
  (set `self.AnimState` "NewEnumerator2")
  (`self.UpdateAnimation`))

(fn `UserConstructionScript`)