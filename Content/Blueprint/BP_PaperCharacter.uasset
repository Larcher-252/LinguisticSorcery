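; BP_PaperCharacter is a 2D Paper character for what appears to be a word-answer game with player HP.
; On BeginPlay it passes its HP percentage to the widget held by HUD_Custom and shows a word.
; Three Answer input actions forward the chosen option number to the HUD through AnswerToHUD.
; An UpdateAnimation event sets the sprite to the idle flipbook.
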(event `self.ReceiveBeginPlay`
  (bind _ashud_custom (cast `/Game/Blueprint/UI/HUD_Custom` (`PlayerController.GetHUD` (`GameplayStatics.GetPlayerController` 0))))
  (bind _hud_ref (`/Game/Blueprint/UI/HUD_Custom.HUD_Ref` _ashud_custom))
  (set `/Game/Blueprint/UI/W_HUD.Player_HP_Percent` (/ (`self.HP_current`) (`self.HP_max`)) _hud_ref)
  (`/Game/Blueprint/UI/W_HUD.Show word` _hud_ref))

(event `InputAction|Pause/Exit`
  (params (Key :type "Key Structure")))

(event `InputAction|Answer1`
  (params (Key :type "Key Structure"))
  (:`Pressed`
    (bind _ashud_custom (cast `/Game/Blueprint/UI/HUD_Custom` (`PlayerController.GetHUD` (`GameplayStatics.GetPlayerController` 0))))
    (`/Game/Blueprint/UI/HUD_Custom.AnswerToHUD` _ashud_custom 1)))

(event `InputAction|Answer2`
  (params (Key :type "Key Structure"))
  (:`Pressed`
    (bind _ashud_custom (cast `/Game/Blueprint/UI/HUD_Custom` (`PlayerController.GetHUD` (`GameplayStatics.GetPlayerController` 0))))
    (`/Game/Blueprint/UI/HUD_Custom.AnswerToHUD` _ashud_custom 2)))

(event `InputAction|Answer3`
  (params (Key :type "Key Structure"))
  (:`Pressed`
    (bind _ashud_custom (cast `/Game/Blueprint/UI/HUD_Custom` (`PlayerController.GetHUD` (`GameplayStatics.GetPlayerController` 0))))
    (`/Game/Blueprint/UI/HUD_Custom.AnswerToHUD` _ashud_custom 3)))

(event `Update Animation`
  (`PaperFlipbookComponent.SetFlipbook` (`self.Sprite`) "/Game/Assets/Sprites/Characters/Idle/FB_Character_Idle.FB_Character_Idle"))

(fn `UserConstructionScript`)